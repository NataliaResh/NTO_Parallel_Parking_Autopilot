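; BP_Parktronic is a parking-sensor actor that measures distance along its forward vector with a line trace.
; Each tick it moves a Sphere to the hit distance or maximum range, draws a colored debug line, and stores the sphere's relative-location length.
; The LineControl flag picks the trace channel and line color at BeginPlay.
; GetValue returns the stored length scaled from centimeters to meters.
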(event EventBeginPlay
  (if (Variables|Default|GetbLineControl)
    (Variables|Default|Setcolor (Class|KismetMathLibrary|LinearColorBlue))
    (Variables|Default|SettraceChannel "TraceTypeQuery4")
    (else
      (Variables|Default|Setcolor (Class|KismetMathLibrary|LinearColorRed))
      (Variables|Default|SettraceChannel "TraceTypeQuery3"))))

(event Collision|EventActorBeginOverlap
  (params (OtherActor :type Actor%20Object%20Reference)))

(event EventTick
  (params (DeltaSeconds :type Float%20%28single-precision%29))
  (bind _returnvalue (Transformation|GetActorLocation))
  (bind _returnvalue_2 (Transformation|GetActorForwardVector))
  (bind _returnvalue_3 (* _returnvalue_2 1e+03))
  (bind _returnvalue_4 (+ _returnvalue_3 _returnvalue))
  (bind (_outhit _returnvalue_5) (Collision|LineTraceByChannel _returnvalue _returnvalue_4 (Variables|Default|GettraceChannel) false 0 "None" true "(R=1.000000,G=0.000000,B=0.000000,A=1.000000)" "(R=0.026884,G=1.000000,B=0.000000,A=1.000000)" 0.0))
  (if _returnvalue_5
    (Variables|Default|SetspherePosition (+ _returnvalue (* _returnvalue_2 (.distance _outhit))))
    (else
      (Variables|Default|SetspherePosition _returnvalue_4)))
  (Transformation|SetWorldLocation (Variables|Default|GetSphere) (Variables|Default|GetspherePosition) false false)
  (Variables|Default|Setvalue (Math|Vector|VectorLength (Variables|/Script/Engine.SceneComponent|GetRelativeLocation (Variables|Default|GetSphere))))
  (Rendering|Debug|DrawDebugLine _returnvalue (Variables|Default|GetspherePosition) (Variables|Default|Getcolor) 0.0 0.0))

(fn ConstructionScript)

(fn GetValue
  (return (* (Variables|Default|Getvalue) 0.01)))