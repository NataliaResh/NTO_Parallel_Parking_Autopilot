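; Toyota Chaser vehicle for a parking test, exposing speed, steering and distance-sensor functions alongside manual input axes.
; Tick chases the set speed by flipping forward/reverse gear at full throttle and applies steering from a queue delayed by angle change.
; EndOfParking arms scoring once stopped: the worst of angle, line and rear-gap scores, zeroed on timeout.
; Box overlap, or nonzero set speed at the end, pauses the game.
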(event OnComponentBeginOverlap(Box)
  (params (OverlappedComponent :type Primitive%20Component%20Object%20Reference) (OtherActor :type Actor%20Object%20Reference) (OtherComp :type Primitive%20Component%20Object%20Reference) (OtherBodyIndex :type Integer) (bFromSweep :type Boolean) (SweepResult :type Hit%20Result%20Structure%20%28by%20ref%29))
  (Utilities|String|LogString "Collision!")
  (Game|SetGamePaused true))

(event EventBeginPlay
  (bind _queue (Variables|Default|Getqueue))
  (bind _parkingsensors (Variables|Default|GetparkingSensors))
  (bind _linesensors (Variables|Default|GetlineSensors))
  (bind _output (Utilities|Array|Get(acopy) _queue))
  (Variables|Default|Settime 0.0)
  (Utilities|Array|Add _parkingsensors (Variables|Default|GetParktronic1))
  (Utilities|Array|Add _parkingsensors (Variables|Default|GetParktronic2))
  (Utilities|Array|Add _parkingsensors (Variables|Default|GetParktronic3))
  (Utilities|Array|Add _parkingsensors (Variables|Default|GetParktronic4))
  (Utilities|Array|Add _parkingsensors (Variables|Default|GetParktronic5))
  (Utilities|Array|Add _parkingsensors (Variables|Default|GetParktronic6))
  (Utilities|Array|Add _parkingsensors (Variables|Default|GetParktronic7))
  (Utilities|Array|Add _parkingsensors (Variables|Default|GetParktronic8))
  (Utilities|Array|Add _linesensors (Variables|Default|GetParktronic9))
  (Utilities|Array|Add _linesensors (Variables|Default|GetParktronic10))
  ;[1 1 1] Update Steering Angle
  (if (Utilities|Array|IsEmpty _queue) :!label _label
    (Utilities|FlowControl|Delay 0.01)
    (goto _label)
    (else
      (bind _output_get (Variables|Default|SettempSteerAngle (Variables|Default|GetcurrentSteerAngle)))
      (Variables|Default|SetcurrentSteerAngle _output)
      (Utilities|FlowControl|Delay (* (Math|Float|Absolute(Float) (- _output _output_get)) 0.4))
      (Utilities|Array|RemoveIndex (Variables|Default|Getqueue))
      (goto _label))))

(event EventTick
  (params (DeltaSeconds :type Float%20%28single-precision%29))
  (bind _vehiclemovementcomponent (Variables|Default|GetVehicleMovementComponent))
  ;[1 1 1] CheckEnd
  (if (Variables|Default|GetbEnd)
    (if (!= (Variables|Default|GetcurrentSettedSpeed) 0.0)
      (Utilities|String|LogString "Car is move!")
      (Utilities|String|LogString "Score: 0")
      (Game|SetGamePaused true)
      (else
        (bind _speed (CallFunction|GetSpeed))
        (if (> (Math|Float|Absolute(Float) _speed) 0.01)
          ;[1 1 1] Update
          (bind _speed_2 (CallFunction|GetSpeed :!label _label))
          (Variables|Default|Settime (+ DeltaSeconds (Variables|Default|Gettime)))
          (if (== (Variables|Default|GetcurrentSettedSpeed) 0.0)
            (if (< (Math|Float|Absolute(Float) _speed_2) 0.1)
              (Class|ChaosVehicleMovementComponent|SetThrottleInput _vehiclemovementcomponent 0.0)
              (else
                (if (< _speed_2 (Variables|Default|GetcurrentSettedSpeed)) :!label _label_2
                  (Class|ChaosVehicleMovementComponent|SetTargetGear _vehiclemovementcomponent 1 false)
                  (else
                    (Class|ChaosVehicleMovementComponent|SetTargetGear _vehiclemovementcomponent -1 false)))
                (Class|ChaosVehicleMovementComponent|SetThrottleInput _vehiclemovementcomponent 1.0)))
            (else
              (goto _label_2)))
          (Class|ChaosVehicleMovementComponent|SetSteeringInput (Variables|Default|GetVehicleMovementComponent) (Variables|Default|GetcurrentSteerAngle))
          (else
            (CallFunction|EndOfParkingImpl)))))
    (else
      (goto _label))))

(event Input|AxisEvents|InputAxisThrotlle
  (params (AxisValue :type Float%20%28single-precision%29))
  ;[1 1 1] Manual
  (Class|ChaosVehicleMovementComponent|SetThrottleInput (Variables|Default|GetVehicleMovementComponent) AxisValue))

(event Input|AxisEvents|InputAxisBrake
  (params (AxisValue :type Float%20%28single-precision%29))
  ;[1 1 1] Manual
  (Class|ChaosVehicleMovementComponent|SetBrakeInput (Variables|Default|GetVehicleMovementComponent) AxisValue))

(event Input|AxisEvents|InputAxisSteering
  (params (AxisValue :type Float%20%28single-precision%29))
  ;[1 1 1] Manual
  (Class|ChaosVehicleMovementComponent|SetSteeringInput (Variables|Default|GetVehicleMovementComponent) AxisValue))

(fn ConstructionScript)

(fn GetSpeed
  (return (* (Vehicle|GetForwardSpeed (Variables|Default|GetVehicleMovementComponent)) 0.036)))

(fn GetSteeringAngle
  (return (- 1.8e+02 (Math|Float|Absolute(Float) (.yaw (Transformation|GetWorldRotation (Variables|Character|GetMesh)))))))

(fn SetSpeed
  (params (value :type Float%20%28double-precision%29))
  (if (> value 6e+01)
    (Variables|Default|SetcurrentSettedSpeed 6e+01)
    (elif (< value -6e+01)
      (Variables|Default|SetcurrentSettedSpeed -6e+01)
      (else
        (Variables|Default|SetcurrentSettedSpeed value)))))

(fn SetSteeringAngle
  (params (value :type Float%20%28double-precision%29))
  (if (> 0.0 1.0)
    (Variables|Default|SetcurrentSteerAngle 1.0)
    (elif (< 0.0 -1.0)
      (Variables|Default|SetcurrentSteerAngle -1.0)
      (else
        (Variables|Default|SetcurrentSteerAngle value))))
  (Utilities|Array|Add (Variables|Default|Getqueue) (Variables|Default|GetcurrentSteerAngle)))

(fn GetParkingSensorDistance
  (params (index :type Integer))
  (bind _parkingsensors (Variables|Default|GetparkingSensors))
  (if (or (>= index (Utilities|Array|Length _parkingsensors)) (< index 0))
    (return -1.0)
    (else
      (bind _asbp_parktronic (Utilities|Casting|CastToBP_Parktronic (Variables|/Script/Engine.ChildActorComponent|GetChildActor (Utilities|Array|Get(acopy) _parkingsensors index))))
      (bind _value (Default|GetValue _asbp_parktronic))
      (return _value))))

(fn GetDistancetoLine
  (params (index :type Integer))
  (if (or (> index 1) (< index 0))
    (return -1.0)
    (else
      (bind _asbp_parktronic (Utilities|Casting|CastToBP_Parktronic (Variables|/Script/Engine.ChildActorComponent|GetChildActor (Utilities|Array|Get(acopy) (Variables|Default|GetlineSensors) index))))
      (bind _value (Default|GetValue _asbp_parktronic))
      (return _value))))

(fn EndOfParking
  (Variables|Default|SetbEnd true))

(fn EndOfParkingImpl
  (bind _time (Variables|Default|Gettime))
  (Utilities|String|LogString "Time: ")
  (Utilities|String|LogString (Utilities|String|ToString(Text) (Utilities|Text|ToText(Float) _time "HalfToEven")))
  (if (> _time 5e+01)
    (Utilities|String|LogString "Time Limit!")
    (else
      (Utilities|String|LogString "Car angle:")
      (bind _angle (CallFunction|GetSteeringAngle))
      (Utilities|String|LogString (Utilities|String|ToString(Float) _angle))
      (if (<= _angle 1.0)
        (LocalVariables|SetangleScore 1.0)
        (else
          (LocalVariables|SetangleScore (/ (- 45.0 _angle) 44.0))))
      (bind _distance (CallFunction|GetDistancetoLine))
      (bind _distance_2 (CallFunction|GetDistancetoLine 1))
      (if (< _distance _distance_2)
        (LocalVariables|SetdistanceToLine _distance)
        (else
          (LocalVariables|SetdistanceToLine _distance_2)))
      (LocalVariables|SetminDistanceToLine (* (Math|Trig|Cos(Degrees) _angle) (LocalVariables|GetdistanceToLine)))
      (Utilities|String|LogString "Distance to line:")
      (Utilities|String|LogString (Utilities|String|ToString(Float) (LocalVariables|GetdistanceToLine)))
      (if (and (< 0.7 (LocalVariables|GetminDistanceToLine)) (< (LocalVariables|GetminDistanceToLine) 3.0))
        (LocalVariables|SetlineScore (/ (- (LocalVariables|GetminDistanceToLine) 0.7) 2.3))
        (elif (>= (LocalVariables|GetminDistanceToLine) 3.0)
          (LocalVariables|SetlineScore 1.0)
          (else
            (LocalVariables|SetlineScore 0.0))))
      (Utilities|String|LogString "Distance to back obstacle:")
      (bind _distance_3 (CallFunction|GetParkingSensorDistance 4))
      (Utilities|String|LogString (Utilities|String|ToString(Float) _distance_3))
      (if (< _distance_3 0.2)
        (LocalVariables|SetdistanceScore (/ _distance_3 0.2))
        (elif (<= _distance_3 0.4)
          (LocalVariables|SetdistanceScore 1.0)
          (elif (< _distance_3 0.6)
            (LocalVariables|SetdistanceScore (/ _distance_3 0.2))
            (else
              (LocalVariables|SetdistanceScore 0.0)))))
      (if (<= (Variables|Default|Gettime) 5e+01)
        (Utilities|String|LogString "Score:")
        (Utilities|String|LogString (Utilities|String|ToString(Float) (* (Math|Float|Min(Float) (Math|Float|Min(Float) (LocalVariables|GetangleScore) (LocalVariables|GetlineScore)) (LocalVariables|GetdistanceScore)) 1e+02)))
        (else
          (Utilities|String|LogString "Score: 0")))
      (Game|SetGamePaused true))))