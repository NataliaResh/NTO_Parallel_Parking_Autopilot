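; BP_Solution is a scripted driving sequence that controls the BP_Toyota_Chaser car through a parking task.
; On BeginPlay it finds the car in the level and, after a brief initial delay, issues timed SetSpeed calls for positive speed, negative speed and stop.
; The sequence is open-loop, using only delays with no position checks, and ends by calling EndOfParking on the car.
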(event EventBeginPlay
  (bind _returnvalue (Actor|GetActorOfClass "/Game/Assets/Toyota/BP_Toyota_Chaser.BP_Toyota_Chaser_C"))
  (Variables|Default|Setcar _returnvalue)
  (Utilities|FlowControl|Delay 0.002)
  (Default|SetSpeed (Variables|Default|Getcar) 1e+01)
  (Utilities|FlowControl|Delay 5.0)
  (Default|SetSpeed (Variables|Default|Getcar) -5.0)
  (Utilities|FlowControl|Delay 5.0)
  (Default|SetSpeed (Variables|Default|Getcar) 0.0)
  (Default|EndOfParking (Variables|Default|Getcar)))

(fn ConstructionScript)